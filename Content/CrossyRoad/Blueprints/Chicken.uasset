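; Player chicken pawn for a Crossy Road clone that hops on input release with squash animation and tracks the furthest row.
; Each new furthest row spawns a row and culls old props.
; Overlaps set log and lily-pad riding, block trees and rocks by restoring the previous location, or trigger vehicle, train and water deaths.
; Idling or retreating too far summons an eagle; deaths save coins and high score, then show the end screen.
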(event `self.ReceiveBeginPlay`
  (bind _asgi_crossy_road (cast `/Game/CrossyRoad/Blueprints/GI_CrossyRoad` (`GameplayStatics.GetGameInstance`)))
  (`/Game/CrossyRoad/Blueprints/GI_CrossyRoad.LoadGame` _asgi_crossy_road)
  (`self.UpdateCoinText`)
  (`self.DisableInput` null))

(event `self.ReceiveActorBeginOverlap`
  (params (OtherActor :type "Actor Object Reference"))
  (if (`self.GameStart`)
    (bind _asv_log (cast `/Game/CrossyRoad/Blueprints/V_Log` OtherActor)
      (:`then`
        (set `self.LogCurrentlyOn` _asv_log)
        (set `self.OnLog` true)
        (`ActorComponent.Activate` (`self.LogSound`) false))
      (:`CastFailed`
        (bind _asv_car (cast `/Game/CrossyRoad/Blueprints/V_Car` OtherActor)
          (:`then`
            (`self.DeathAnimation` 0 _asv_car)
            (`self.ResetGame` :!label _label))
          (:`CastFailed`
            (bind _asv_truck (cast `/Game/CrossyRoad/Blueprints/V_Truck` OtherActor)
              (:`then`
                (`self.DeathAnimation` 0 null _asv_truck)
                (goto _label))
              (:`CastFailed`
                (cast `/Game/CrossyRoad/Blueprints/V_Train` OtherActor
                  (:`then`
                    (`self.DeathAnimation` 1)
                    (goto _label))
                  (:`CastFailed`
                    (cast `/Game/CrossyRoad/Blueprints/E_Tree` OtherActor
                      (:`then`
                        (`SceneComponent.K2_SetWorldLocation` (`self.Scene`) (`self.PreviousLocation`) false false :!label _label_2))
                      (:`CastFailed`
                        (cast `/Game/CrossyRoad/Blueprints/E_Rock` OtherActor
                          (:`then`
                            (goto _label_2))
                          (:`CastFailed`
                            (cast `/Game/CrossyRoad/Blueprints/Tile_Row` OtherActor
                              (:`then`
                                (set `self.OnWater` true))
                              (:`CastFailed`
                                (cast `/Game/CrossyRoad/Blueprints/E_LilyPad` OtherActor
                                  (:`then`
                                    (set `self.OnLily` true)
                                    (`ActorComponent.Activate` (`self.LilySound`) false))
                                  (:`CastFailed`
                                    (cast `/Game/CrossyRoad/Blueprints/Coin` OtherActor)
                                    (`ActorComponent.Activate` (`self.CoinSound`) false)))))))))))))))))))

(event `self.ReceiveActorEndOverlap`
  (params (OtherActor :type "Actor Object Reference"))
  (cast `/Game/CrossyRoad/Blueprints/V_Log` OtherActor
    (:`then`
      (set `self.OnLog` false)
      (for _ (`self.GetOverlappingActors` "/Game/CrossyRoad/Blueprints/V_Log.V_Log_C")
        (set `self.OnLog` true)
        (`ActorComponent.Activate` (`self.LogSound`) false)))
    (:`CastFailed`
      (cast `/Game/CrossyRoad/Blueprints/Tile_Row` OtherActor
        (:`then`
          (set `self.OnWater` false))
        (:`CastFailed`
          (cast `/Game/CrossyRoad/Blueprints/E_LilyPad` OtherActor)
          (set `self.OnLily` false))))))

(event `self.ReceiveTick`
  (params (DeltaSeconds :type "Float (single-precision)"))
  (`self.EagleMovement`)
  (`self.VehicleMovement`)
  (if (`self.GameStart`)
    (if (>= (`self.IdleTime`) 10.0)
      (if (`self.EagleSpawned`) :!label _label_3
        (`self.SpawnEagle`)
        (`self.ResetGame`))
      (elif (>= (- (`self.FurthestTileNumber`) (`self.CurrentTileNumber`)) 7)
        (goto _label_3)
        (else
          (set `self.IdleTime` (+ DeltaSeconds (`self.IdleTime`)))
          (if (`self.OnWater`)
            (if (`self.OnLog`)
              (`self.DecideMovement` :!label _label_4)
              (elif (`self.OnLily`)
                (goto _label_4)
                (else
                  (`self.DeathAnimation` 2)
                  (`self.ResetGame`))))
            (else
              (goto _label_4))))))))

(event `InputAction|MoveForward`
  (params (Key :type "Key Structure"))
  (bind _staticmesh (`self.StaticMesh`))
  (bind _staticmesh_2 (`self.StaticMesh`))
  (:`Pressed`
    (`SceneComponent.SetRelativeScale3D` _staticmesh (1.0 1.0 0.8))
    (`SceneComponent.K2_AddLocalOffset` _staticmesh_2 (0.0 0.0 -5.0) false false))
  (:`Released`
    (`SceneComponent.SetRelativeScale3D` _staticmesh (1.0 1.0 1.0))
    (`SceneComponent.K2_AddLocalOffset` _staticmesh_2 (0.0 0.0 5.0) false false)
    (`SceneComponent.K2_AddLocalOffset` (`self.StaticMesh`) (0.0 0.0 30.0) false false)
    (`self.AddMovementInput` (`self.GetActorForwardVector`) 40.0)
    (`SceneComponent.K2_SetRelativeRotation` :`self` (`self.StaticMesh`))
    (`self.IncreaseCurrentTile`)
    (set `self.IdleTime` 0.0)
    (`ActorComponent.Activate` (`self.MoveSound`) false)))

(event `InputAction|MoveBackward`
  (params (Key :type "Key Structure"))
  (bind _staticmesh (`self.StaticMesh`))
  (bind _staticmesh_2 (`self.StaticMesh`))
  (:`Pressed`
    (`SceneComponent.SetRelativeScale3D` _staticmesh (1.0 1.0 0.8))
    (`SceneComponent.K2_AddLocalOffset` _staticmesh_2 (0.0 0.0 -5.0) false false))
  (:`Released`
    (`SceneComponent.SetRelativeScale3D` _staticmesh (1.0 1.0 1.0))
    (`SceneComponent.K2_AddLocalOffset` _staticmesh_2 (0.0 0.0 5.0) false false)
    (`SceneComponent.K2_AddLocalOffset` (`self.StaticMesh`) (0.0 0.0 30.0) false false)
    (`self.AddMovementInput` (`self.GetActorForwardVector`) -40.0)
    (`SceneComponent.K2_SetRelativeRotation` (`self.StaticMesh`) (struct :`Yaw` 180.0) false false)
    (`self.DecreaseCurrentTile`)
    (set `self.IdleTime` 0.0)
    (`ActorComponent.Activate` (`self.MoveSound`) false)))

(event `InputAction|MoveRight`
  (params (Key :type "Key Structure"))
  (bind _staticmesh (`self.StaticMesh`))
  (bind _staticmesh_2 (`self.StaticMesh`))
  (:`Pressed`
    (`SceneComponent.SetRelativeScale3D` _staticmesh (1.0 1.0 0.8))
    (`SceneComponent.K2_AddLocalOffset` _staticmesh_2 (0.0 0.0 -5.0) false false))
  (:`Released`
    (`SceneComponent.SetRelativeScale3D` _staticmesh (1.0 1.0 1.0))
    (`SceneComponent.K2_AddLocalOffset` _staticmesh_2 (0.0 0.0 5.0) false false)
    (`SceneComponent.K2_AddLocalOffset` (`self.StaticMesh`) (0.0 0.0 30.0) false false)
    (`self.AddMovementInput` (`self.GetActorRightVector`) 40.0)
    (`SceneComponent.K2_SetRelativeRotation` (`self.StaticMesh`) (struct :`Yaw` 90.0) false false)
    (set `self.IdleTime` 0.0)
    (`ActorComponent.Activate` (`self.MoveSound`) false)))

(event `InputAction|MoveLeft`
  (params (Key :type "Key Structure"))
  (bind _staticmesh (`self.StaticMesh`))
  (bind _staticmesh_2 (`self.StaticMesh`))
  (:`Pressed`
    (`SceneComponent.SetRelativeScale3D` _staticmesh (1.0 1.0 0.8))
    (`SceneComponent.K2_AddLocalOffset` _staticmesh_2 (0.0 0.0 -5.0) false false))
  (:`Released`
    (`SceneComponent.SetRelativeScale3D` _staticmesh (1.0 1.0 1.0))
    (`SceneComponent.K2_AddLocalOffset` _staticmesh_2 (0.0 0.0 5.0) false false)
    (`SceneComponent.K2_AddLocalOffset` (`self.StaticMesh`) (0.0 0.0 30.0) false false)
    (`self.AddMovementInput` (`self.GetActorRightVector`) -40.0)
    (`SceneComponent.K2_SetRelativeRotation` (`self.StaticMesh`) (struct :`Yaw` -90.0) false false)
    (set `self.IdleTime` 0.0)
    (`ActorComponent.Activate` (`self.MoveSound`) false)))

(fn `DeathAnimation`
  (params (DeathType :type Integer) (Car :type "/Game/CrossyRoad/Blueprints/V_Car Object Reference") (Truck :type "/Game/CrossyRoad/Blueprints/V_Truck Object Reference"))
  (bind (_returnvalue_x _returnvalue_y) (`KismetMathLibrary.BreakVector` (`self.K2_GetActorLocation` Car)))
  (bind (_returnvalue_x_2 _returnvalue_y_2) (`KismetMathLibrary.BreakVector` (`self.K2_GetActorLocation`)))
  (bind (_returnvalue_x_3 _returnvalue_y_3) (`KismetMathLibrary.BreakVector` (`self.K2_GetActorLocation` Truck)))
  (bind (_returnvalue_x_4 _returnvalue_y_4 _returnvalue_z) (`KismetMathLibrary.BreakVector` (`SceneComponent.K2_GetComponentLocation` (`self.StaticMesh`))))
  (switch `int` DeathType
    (:`0`
      (`/Engine/EditorBlueprintResources/StandardMacros.IsValid` Car
        (:`Is Valid`
          (set `self.Car` Car)
          (if (`KismetMathLibrary.NearlyEqual_FloatFloat` _returnvalue_y _returnvalue_y_2 20.0)
            (`SceneComponent.SetRelativeScale3D` (`self.StaticMesh`) (0.1 1.0 1.0) :!label _label)
            (`SceneComponent.K2_AddLocalOffset` (`self.StaticMesh`) (-15.0 0.0 0.0) false false)
            (set `self.OnCar` true)
            (else
              (if (>= _returnvalue_z 25.0) :!label _label_2
                (`SceneComponent.K2_AddLocalOffset` (`self.StaticMesh`) (0.0 0.0 -30.0) false false))
              (`SceneComponent.SetRelativeScale3D` (`self.StaticMesh`) (1.0 1.0 0.1))
              (`SceneComponent.K2_AddLocalOffset` (`self.StaticMesh`) (0.0 0.0 -15.0) false false))))
        (:`Is Not Valid`
          (`/Engine/EditorBlueprintResources/StandardMacros.IsValid` Truck
            (:`Is Valid`
              (set `self.Truck` Truck)
              (if (`KismetMathLibrary.NearlyEqual_FloatFloat` _returnvalue_y_2 _returnvalue_y_3 20.0)
                (goto _label)
                (else
                  (goto _label_2))))))))
    (:`1`
      (`ActorComponent.Activate` (`self.DeathExplosion`) false)
      (`SceneComponent.SetVisibility` (`self.StaticMesh`) false false))
    (:`2`
      (`SceneComponent.K2_AddLocalOffset` (`self.StaticMesh`) (0.0 0.0 -100.0) false false)
      (`ActorComponent.Activate` (`self.WaterSplash`) false)
      (`ActorComponent.Activate` (`self.WaterSound`) false))))

(fn `DecideMovement`
  (bind (_returnvalue_x _returnvalue_y _returnvalue_z) (`KismetMathLibrary.BreakVector` (`SceneComponent.K2_GetComponentLocation` (`self.StaticMesh`))))
  (set `self.PreviousLocation` (`SceneComponent.K2_GetComponentLocation` (`self.Scene`)))
  (if (`self.OnLog`)
    (`self.K2_AddActorLocalOffset` (`KismetMathLibrary.MakeVector` 0.0 (`/Game/CrossyRoad/Blueprints/V_Log.Speed` (`self.LogCurrentlyOn`))) true)
    (bind _returnvalue (`self.ConsumeMovementInputVector`))
    (`self.K2_AddActorLocalOffset` _returnvalue true)
    (else
      (bind _returnvalue_2 (`self.ConsumeMovementInputVector`))
      (`self.K2_AddActorLocalOffset` _returnvalue_2 true)))
  (if (>= _returnvalue_z 30.0)
    (`SceneComponent.K2_AddLocalOffset` (`self.StaticMesh`) (0.0 0.0 -10.0) false false)))

(fn `DecreaseCurrentTile`
  (bind _result (`/Engine/EditorBlueprintResources/StandardMacros.DecrementInt` (`self.CurrentTileNumber`))
    (:`  `
      (set `self.CurrentTileNumber` _result))))

(fn `EagleMovement`
  (bind _returnvalue_x (`KismetMathLibrary.BreakVector` (`self.K2_GetActorLocation`)))
  (bind _eagle (`self.Eagle`))
  (bind _returnvalue_x_2 (`KismetMathLibrary.BreakVector` (`self.K2_GetActorLocation` _eagle)))
  (bind (_returnvalue_x_3 _returnvalue_y _returnvalue_z) (`KismetMathLibrary.BreakVector` (`SceneComponent.K2_GetComponentLocation` (`self.StaticMesh`))))
  (if (not (`self.EagleSpawned`))
    (if (>= _returnvalue_z 30.0)
      (`SceneComponent.K2_AddLocalOffset` (`self.StaticMesh`) (0.0 0.0 -10.0) false false))
    (if (<= _returnvalue_x_2 _returnvalue_x)
      (`SceneComponent.K2_AddWorldOffset` (`self.StaticMesh`) (`KismetMathLibrary.MakeVector` (`/Game/CrossyRoad/Blueprints/Eagle.Speed` _eagle) 0.0 0.5) false false))))

(fn `IncreaseCurrentTile`
  (bind _returnvalue_x (`KismetMathLibrary.BreakVector` (`self.K2_GetActorLocation`)))
  (bind _returnvalue_x_2 (`KismetMathLibrary.BreakVector` (`self.K2_GetActorLocation`)))
  (bind _returnvalue_x_3 (`KismetMathLibrary.BreakVector` (`self.K2_GetActorLocation`)))
  (bind _returnvalue_x_4 (`KismetMathLibrary.BreakVector` (`self.K2_GetActorLocation`)))
  (bind _furthesttilenumber (`self.FurthestTileNumber`))
  (bind _result (`/Engine/EditorBlueprintResources/StandardMacros.IncrementInt` (`self.CurrentTileNumber`))
    (:`  `
      (bind _output_get (set `self.CurrentTileNumber` _result))
      (if (> _output_get (`self.FurthestTileNumber`))
        (set `self.FurthestTileNumber` (`self.CurrentTileNumber`))
        (if (> _furthesttilenumber (`self.HighScore`))
          (set `self.HighScore` _furthesttilenumber))
        (`self.UpdateStepText`)
        (`/Game/CrossyRoad/Blueprints/Spawner_Row.SpawnRowAtSpawnPoint` (`self.RowSpawner`))
        (bind _outactors (`GameplayStatics.GetAllActorsOfClass` "/Game/CrossyRoad/Blueprints/Tile_Row.Tile_Row_C"))
        (for _array_element _outactors
          (`/Game/CrossyRoad/Blueprints/Tile_Row.DestroyRow` _array_element))
        (bind _outactors_2 (`GameplayStatics.GetAllActorsOfClass` "/Game/CrossyRoad/Blueprints/E_Rock.E_Rock_C"))
        (for _array_element_2 _outactors_2
          (bind _returnvalue_x_5 (`KismetMathLibrary.BreakVector` (`self.K2_GetActorLocation` _array_element_2)))
          (if (>= _returnvalue_x (+ _returnvalue_x_5 400.0))
            (`self.K2_DestroyActor` _array_element_2)))
        (bind _outactors_3 (`GameplayStatics.GetAllActorsOfClass` "/Game/CrossyRoad/Blueprints/E_Tree.E_Tree_C"))
        (for _array_element_3 _outactors_3
          (bind _returnvalue_x_6 (`KismetMathLibrary.BreakVector` (`self.K2_GetActorLocation` _array_element_3)))
          (if (>= _returnvalue_x_3 (+ _returnvalue_x_6 400.0))
            (`self.K2_DestroyActor` _array_element_3)))
        (bind _outactors_4 (`GameplayStatics.GetAllActorsOfClass` "/Game/CrossyRoad/Blueprints/Coin.Coin_C"))
        (for _array_element_4 _outactors_4
          (bind _returnvalue_x_7 (`KismetMathLibrary.BreakVector` (`self.K2_GetActorLocation` _array_element_4)))
          (if (>= _returnvalue_x_4 (+ _returnvalue_x_7 400.0))
            (`self.K2_DestroyActor` _array_element_4)))
        (bind _outactors_5 (`GameplayStatics.GetAllActorsOfClass` "/Game/CrossyRoad/Blueprints/E_LilyPad.E_LilyPad_C"))
        (for _array_element_5 _outactors_5
          (bind _returnvalue_x_8 (`KismetMathLibrary.BreakVector` (`self.K2_GetActorLocation` _array_element_5)))
          (if (>= _returnvalue_x_2 (+ _returnvalue_x_8 400.0))
            (`self.K2_DestroyActor` _array_element_5)))))))

(fn `ResetGame`
  (bind _asgi_crossy_road (cast `/Game/CrossyRoad/Blueprints/GI_CrossyRoad` (`GameplayStatics.GetGameInstance`)))
  (`/Game/CrossyRoad/Blueprints/GI_CrossyRoad.SaveGame` _asgi_crossy_road (`self.CoinsCollected`) (`self.HighScore`))
  (`/Game/CrossyRoad/Blueprints/GM_CrossyRoad.ShowEndScreen` (`self.GM_CrossyRoad`)))

(fn `SpawnEagle`
  (bind (_returnvalue_x _returnvalue_y) (`KismetMathLibrary.BreakVector` (`SceneComponent.K2_GetComponentLocation` (`self.Scene`))))
  (set `self.EagleSpawned` false)
  (bind _returnvalue (`|SpawnActorFromClass` "/Game/CrossyRoad/Blueprints/Eagle.Eagle_C" (`KismetMathLibrary.MakeTransform` (`KismetMathLibrary.MakeVector` (+ _returnvalue_x 400.0) _returnvalue_y 75.0)) "Undefined" "OverrideRootScale" null null))
  (set `self.Eagle` _returnvalue))

(fn `UpdateCoinText`
  (bind _gameinterface (`self.GameInterface`))
  (`/Engine/EditorBlueprintResources/StandardMacros.IsValid` _gameinterface
    (:`Is Valid`
      (`/Game/CrossyRoad/UI/GameInterface.UpdateCoinText` _gameinterface (`self.CoinsCollected`)))))

(fn `UpdateStepText`
  (bind _gameinterface (`self.GameInterface`))
  (`/Engine/EditorBlueprintResources/StandardMacros.IsValid` _gameinterface
    (:`Is Valid`
      (`/Game/CrossyRoad/UI/GameInterface.UpdateStepText` _gameinterface (`self.FurthestTileNumber`)))))

(fn `UserConstructionScript`)

(fn `VehicleMovement`
  (bind _car (`self.Car`))
  (bind _truck (`self.Truck`))
  (if (`self.OnCar`)
    (`/Engine/EditorBlueprintResources/StandardMacros.IsValid` _car
      (:`Is Valid`
        (`SceneComponent.K2_AddWorldOffset` (`self.StaticMesh`) (`KismetMathLibrary.MakeVector` 0.0 (`/Game/CrossyRoad/Blueprints/V_Car.Speed` _car)) false false))
      (:`Is Not Valid`
        (`/Engine/EditorBlueprintResources/StandardMacros.IsValid` _truck
          (:`Is Valid`
            (`SceneComponent.K2_AddWorldOffset` (`self.StaticMesh`) (`KismetMathLibrary.MakeVector` 0.0 (`/Game/CrossyRoad/Blueprints/V_Truck.Speed` _truck)) false false)))))))