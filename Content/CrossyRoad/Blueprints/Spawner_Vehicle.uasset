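; Vehicle spawner for a Crossy Road-style tile row, sending cars or trucks, logs, or trains across it by RowType.
; BeginPlay picks one random Direction, which sets the spawn side and is passed to each vehicle's setup.
; Tick accumulates time against a per-type random interval, re-rolled every frame, then spawns and resets.
; Train spawns also start the row's TrainPost lights, but enable its sound only when Direction is true.
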(event `self.ReceiveBeginPlay`
  (set `self.Direction` (`KismetMathLibrary.RandomBool`)))

(event `self.ReceiveTick`
  (params (DeltaSeconds :type "Float (single-precision)"))
  (switch `int` (`self.RowType`)
    (:`1`
      _)
    (:`2`
      _)
    (:`3`
      _))
  (bind _output_get (set `self.Counter` (+ DeltaSeconds (`self.Counter`))))
  (if (>= _output_get (select `int` (`self.RowType`) :`0` 0.0 :`1` (`KismetMathLibrary.RandomFloatInRange` 3.0 5.0) :`2` (`KismetMathLibrary.RandomFloatInRange` 3.0 4.0) :`3` (`KismetMathLibrary.RandomFloatInRange` 10.0 15.0)))
    (switch `int` (`self.RowType`)
      (:`1`
        (`/Engine/EditorBlueprintResources/StandardMacros.IsValid` self
          (:`Is Valid`
            (`self.SpawnCar`))))
      (:`2`
        (`/Engine/EditorBlueprintResources/StandardMacros.IsValid` self
          (:`Is Valid`
            (`self.SpawnLog`))))
      (:`3`
        (`/Engine/EditorBlueprintResources/StandardMacros.IsValid` self
          (:`Is Valid`
            (`self.SpawnTrain`)))))
    (set `self.Counter` 0.0)))

(fn `SpawnCar`
  (bind _direction (`self.Direction`))
  (bind _returnvalue_x (`KismetMathLibrary.BreakVector` (`self.K2_GetActorLocation` (`self.TileRow`))))
  (switch `int` (`KismetMathLibrary.RandomIntegerInRange` 0 1)
    (:`0`
      (if (`self.Direction`)
        (bind _returnvalue (`|SpawnActorFromClass` "/Game/CrossyRoad/Blueprints/V_Car.V_Car_C" (`KismetMathLibrary.MakeTransform` (`KismetMathLibrary.MakeVector` _returnvalue_x -700.0 3.5)) "Undefined" "OverrideRootScale" null null))
        (`/Engine/EditorBlueprintResources/StandardMacros.IsValid` _returnvalue
          (:`Is Valid`
            (set `/Game/CrossyRoad/Blueprints/V_Car.Direction` _direction _returnvalue)
            (`/Game/CrossyRoad/Blueprints/V_Car.SetupCar` _returnvalue)))
        (else
          (bind _returnvalue_2 (`|SpawnActorFromClass` "/Game/CrossyRoad/Blueprints/V_Car.V_Car_C" (`KismetMathLibrary.MakeTransform` (`KismetMathLibrary.MakeVector` _returnvalue_x 700.0 3.5)) "Undefined" "OverrideRootScale" null null))
          (`/Engine/EditorBlueprintResources/StandardMacros.IsValid` _returnvalue_2
            (:`Is Valid`
              (set `/Game/CrossyRoad/Blueprints/V_Car.Direction` _direction _returnvalue_2)
              (`/Game/CrossyRoad/Blueprints/V_Car.SetupCar` _returnvalue_2))))))
    (:`1`
      (if (`self.Direction`)
        (bind _returnvalue_3 (`|SpawnActorFromClass` "/Game/CrossyRoad/Blueprints/V_Truck.V_Truck_C" (`KismetMathLibrary.MakeTransform` (`KismetMathLibrary.MakeVector` _returnvalue_x -700.0 3.5)) "Undefined" "OverrideRootScale" null null))
        (`/Engine/EditorBlueprintResources/StandardMacros.IsValid` _returnvalue_3
          (:`Is Valid`
            (set `/Game/CrossyRoad/Blueprints/V_Truck.Direction` _direction _returnvalue_3)
            (`/Game/CrossyRoad/Blueprints/V_Truck.SetupTruck` _returnvalue_3)))
        (else
          (bind _returnvalue_4 (`|SpawnActorFromClass` "/Game/CrossyRoad/Blueprints/V_Truck.V_Truck_C" (`KismetMathLibrary.MakeTransform` (`KismetMathLibrary.MakeVector` _returnvalue_x 700.0 3.5)) "Undefined" "OverrideRootScale" null null))
          (`/Engine/EditorBlueprintResources/StandardMacros.IsValid` _returnvalue_4
            (:`Is Valid`
              (set `/Game/CrossyRoad/Blueprints/V_Truck.Direction` _direction _returnvalue_4)
              (`/Game/CrossyRoad/Blueprints/V_Truck.SetupTruck` _returnvalue_4))))))))

(fn `SpawnLog`
  (bind _returnvalue_x (`KismetMathLibrary.BreakVector` (`self.K2_GetActorLocation` (`self.TileRow`))))
  (if (`self.Direction`)
    (bind _returnvalue (`|SpawnActorFromClass` "/Game/CrossyRoad/Blueprints/V_Log.V_Log_C" (`KismetMathLibrary.MakeTransform` (`KismetMathLibrary.MakeVector` _returnvalue_x -1000.0 1.5)) "Undefined" "OverrideRootScale" null null))
    (`/Engine/EditorBlueprintResources/StandardMacros.IsValid` _returnvalue
      (:`Is Valid`
        (set `/Game/CrossyRoad/Blueprints/V_Log.Direction` (`self.Direction`) _returnvalue)
        (`/Game/CrossyRoad/Blueprints/V_Log.SetupLog` _returnvalue)))
    (else
      (bind _returnvalue_2 (`|SpawnActorFromClass` "/Game/CrossyRoad/Blueprints/V_Log.V_Log_C" (`KismetMathLibrary.MakeTransform` (`KismetMathLibrary.MakeVector` _returnvalue_x 1000.0 1.5)) "Undefined" "OverrideRootScale" null null))
      (`/Engine/EditorBlueprintResources/StandardMacros.IsValid` _returnvalue_2
        (:`Is Valid`
          (set `/Game/CrossyRoad/Blueprints/V_Log.Direction` (`self.Direction`) _returnvalue_2)
          (`/Game/CrossyRoad/Blueprints/V_Log.SetupLog` _returnvalue_2))))))

(fn `SpawnTrain`
  (bind _direction (`self.Direction`))
  (bind _returnvalue_x (`KismetMathLibrary.BreakVector` (`self.K2_GetActorLocation` (`self.TileRow`))))
  (bind _trainpost (`/Game/CrossyRoad/Blueprints/Tile_Row.TrainPost` (`self.TileRow`)))
  (bind _trainpost_2 (`/Game/CrossyRoad/Blueprints/Tile_Row.TrainPost` (`self.TileRow`)))
  (if (`self.Direction`)
    (bind _returnvalue (`|SpawnActorFromClass` "/Game/CrossyRoad/Blueprints/V_Train.V_Train_C" (`KismetMathLibrary.MakeTransform` (`KismetMathLibrary.MakeVector` _returnvalue_x -1200.0 5.5)) "Undefined" "OverrideRootScale" null null))
    (`/Engine/EditorBlueprintResources/StandardMacros.IsValid` _returnvalue
      (:`Is Valid`
        (set `/Game/CrossyRoad/Blueprints/V_Train.Direction` _direction _returnvalue)
        (`/Game/CrossyRoad/Blueprints/V_Train.SetupTrain` _returnvalue)
        (set `/Game/CrossyRoad/Blueprints/Train_Post.BlinkLights` true _trainpost_2)
        (set `/Game/CrossyRoad/Blueprints/Train_Post.SoundOn` true _trainpost_2)
        (set `/Game/CrossyRoad/Blueprints/V_Train.TrainPost` _trainpost_2 _returnvalue)))
    (else
      (bind _returnvalue_2 (`|SpawnActorFromClass` "/Game/CrossyRoad/Blueprints/V_Train.V_Train_C" (`KismetMathLibrary.MakeTransform` (`KismetMathLibrary.MakeVector` _returnvalue_x 1200.0 5.5)) "Undefined" "OverrideRootScale" null null))
      (`/Engine/EditorBlueprintResources/StandardMacros.IsValid` _returnvalue_2
        (:`Is Valid`
          (set `/Game/CrossyRoad/Blueprints/V_Train.Direction` _direction _returnvalue_2)
          (`/Game/CrossyRoad/Blueprints/V_Train.SetupTrain` _returnvalue_2)
          (set `/Game/CrossyRoad/Blueprints/Train_Post.BlinkLights` true _trainpost)
          (set `/Game/CrossyRoad/Blueprints/V_Train.TrainPost` _trainpost _returnvalue_2))))))

(fn `UserConstructionScript`)