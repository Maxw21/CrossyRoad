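; Game mode for a Crossy Road style game that runs the menu flow around the Chicken pawn.
; On BeginPlay it links itself to the Chicken, adds the in-game interface and shows the start screen.
; Menu widgets get a reference back to it to switch between start, character select and end screens.
; It toggles Chicken input and cursor for play, fills end-screen scores from the Chicken and restarts on dismissal.
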(event `self.ReceiveBeginPlay`
  (set `PlayerController.bShowMouseCursor` true (`GameplayStatics.GetPlayerController` 0))
  (bind _aschicken (cast `/Game/CrossyRoad/Blueprints/Chicken` (`GameplayStatics.GetPlayerPawn` 0)))
  (set `/Game/CrossyRoad/Blueprints/Chicken.GM_CrossyRoad` self _aschicken)
  (bind _returnvalue (`|CreateWidget` "/Game/CrossyRoad/UI/GameInterface.GameInterface_C"))
  (`UserWidget.AddToViewport` _returnvalue 0)
  (set `/Game/CrossyRoad/Blueprints/Chicken.GameInterface` _returnvalue _aschicken)
  (bind _returnvalue_2 (`|CreateWidget` "/Game/CrossyRoad/UI/StartScreen.StartScreen_C"))
  (set `self.StartScreen` _returnvalue_2)
  (`UserWidget.AddToViewport` _returnvalue_2 0)
  (set `/Game/CrossyRoad/UI/StartScreen.GameManager` self _returnvalue_2))

(fn `HideCharacterSelectScreen`
  (`Widget.RemoveFromParent` (`self.CharacterSelectScreen`))
  (bind _aschicken (cast `/Game/CrossyRoad/Blueprints/Chicken` (`GameplayStatics.GetPlayerPawn` 0)))
  (`self.EnableInput` _aschicken null)
  (set `/Game/CrossyRoad/Blueprints/Chicken.GameStart` true _aschicken)
  (set `PlayerController.bShowMouseCursor` false (`GameplayStatics.GetPlayerController` 0)))

(fn `HideEndScreen`
  (`self.RestartGame`))

(fn `HideStartScreen`
  (`Widget.RemoveFromParent` (`self.StartScreen`))
  (bind _returnvalue (`|CreateWidget` "/Game/CrossyRoad/UI/CharacterSelectScreen.CharacterSelectScreen_C"))
  (`UserWidget.AddToViewport` _returnvalue 0)
  (set `self.CharacterSelectScreen` _returnvalue)
  (set `/Game/CrossyRoad/UI/CharacterSelectScreen.GameManager` self _returnvalue))

(fn `ShowEndScreen`
  (bind _aschicken (cast `/Game/CrossyRoad/Blueprints/Chicken` (`GameplayStatics.GetPlayerPawn` 0)))
  (`self.DisableInput` _aschicken null)
  (set `/Game/CrossyRoad/Blueprints/Chicken.GameStart` false _aschicken)
  (bind _returnvalue (`|CreateWidget` "/Game/CrossyRoad/UI/EndScreen.EndScreen_C"))
  (`UserWidget.AddToViewport` _returnvalue 0)
  (set `self.EndScreen` _returnvalue)
  (set `/Game/CrossyRoad/UI/EndScreen.GameManager` self _returnvalue)
  (`/Game/CrossyRoad/UI/EndScreen.UpdateScore` _returnvalue (`/Game/CrossyRoad/Blueprints/Chicken.FurthestTileNumber` _aschicken))
  (`/Game/CrossyRoad/UI/EndScreen.UpdateHighScore` _returnvalue (`/Game/CrossyRoad/Blueprints/Chicken.HighScore` _aschicken))
  (set `PlayerController.bShowMouseCursor` true (`GameplayStatics.GetPlayerController` 0)))

(fn `ShowStartScreen`
  (`Widget.RemoveFromParent` (`self.CharacterSelectScreen`))
  (`UserWidget.AddToViewport` (`self.StartScreen`) 0))

(fn `UserConstructionScript`)