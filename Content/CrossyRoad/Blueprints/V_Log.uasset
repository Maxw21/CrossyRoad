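; V_Log is a moving log actor for a Crossy Road style game that drifts along the Y axis and removes itself at the far side.
; SetupLog uses the Direction flag to set a signed speed and end coordinate, then picks one of four log meshes at random.
; Each Tick offsets the actor locally by that speed, without delta-time scaling, and DestroyCheck destroys it once its world Y passes the end coordinate.
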(event `self.ReceiveTick`
  (params (DeltaSeconds :type "Float (single-precision)"))
  (`self.K2_AddActorLocalOffset` (`KismetMathLibrary.MakeVector` 0.0 (`self.Speed`)))
  (`self.DestroyCheck`))

(fn `DestroyCheck`
  (bind (_returnvalue_x _returnvalue_y) (`KismetMathLibrary.BreakVector` (`self.K2_GetActorLocation`)))
  (bind (_returnvalue_x_2 _returnvalue_y_2) (`KismetMathLibrary.BreakVector` (`self.K2_GetActorLocation`)))
  (if (`self.Direction`)
    (if (>= _returnvalue_y (`self.Destination`))
      (`self.K2_DestroyActor`))
    (elif (<= _returnvalue_y_2 (`self.Destination`))
      (`self.K2_DestroyActor`))))

(fn `SetupLog`
  (if (`self.Direction`)
    (set `self.Speed` 2.5)
    (set `self.Destination` 1000.0)
    (else
      (set `self.Speed` -2.5)
      (set `self.Destination` -1000.0)))
  (`StaticMeshComponent.SetStaticMesh` (`self.StaticMesh`) (select `int` (`KismetMathLibrary.RandomIntegerInRange` 0 3) :`0` "/Game/CrossyRoad/Meshes/Environment/Log_1/log_1.log_1" :`1` "/Game/CrossyRoad/Meshes/Environment/Log_2/log_2.log_2" :`2` "/Game/CrossyRoad/Meshes/Environment/Log_3/log_3.log_3" :`3` "/Game/CrossyRoad/Meshes/Environment/Log_4/log_4.log_4" :!type "StaticMesh Object Reference")))

(fn `UserConstructionScript`)