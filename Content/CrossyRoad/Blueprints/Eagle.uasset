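; Eagle actor for the Crossy Road game that flies along its local forward axis with its own sound.
; BeginPlay calls Activate on the eagle sound.
; Each Tick moves it by Speed, climbing slightly while its world X is within a small tolerance of the player pawn's and descending otherwise.
; The offsets are applied per frame without delta-time scaling.
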(event `self.ReceiveBeginPlay`
  (`ActorComponent.Activate` (`self.EagleSound`) false))

(event `self.ReceiveTick`
  (params (DeltaSeconds :type "Float (single-precision)"))
  (bind _returnvalue_x (`KismetMathLibrary.BreakVector` (`self.K2_GetActorLocation`)))
  (bind _speed (`self.Speed`))
  (bind _returnvalue_x_2 (`KismetMathLibrary.BreakVector` (`self.K2_GetActorLocation` (`GameplayStatics.GetPlayerPawn` 0))))
  (if (`KismetMathLibrary.NearlyEqual_FloatFloat` _returnvalue_x _returnvalue_x_2 10.0)
    (`self.K2_AddActorLocalOffset` (`KismetMathLibrary.MakeVector` _speed 0.0 0.5))
    (else
      (`self.K2_AddActorLocalOffset` (`KismetMathLibrary.MakeVector` _speed 0.0 -0.5)))))

(fn `UserConstructionScript`)