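; V_Car is a Crossy Road style traffic vehicle that drives along the Y axis and destroys itself past its lane end.
; SetupCar randomly picks a short or long car mesh, then sets speed, destination and facing from Direction.
; Tick moves it by a fixed per-frame offset, without delta time.
; On roughly 5% of ticks it honks if near the player and runs DestroyCheck against the destination.
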(event `self.ReceiveTick`
  (params (DeltaSeconds :type "Float (single-precision)"))
  (bind (_returnvalue_x _returnvalue_y) (`KismetMathLibrary.BreakVector` (`self.K2_GetActorLocation`)))
  (bind (_returnvalue_x_2 _returnvalue_y_2) (`KismetMathLibrary.BreakVector` (`self.K2_GetActorLocation` (`GameplayStatics.GetPlayerPawn` 0))))
  (`self.K2_AddActorLocalOffset` (`KismetMathLibrary.MakeVector` 0.0 (`self.Speed`)))
  (if (>= (`KismetMathLibrary.RandomIntegerInRange` 0 1000) 950)
    (if (and (`KismetMathLibrary.NearlyEqual_FloatFloat` _returnvalue_x _returnvalue_x_2 45.0) (`KismetMathLibrary.NearlyEqual_FloatFloat` _returnvalue_y _returnvalue_y_2 45.0))
      (`ActorComponent.Activate` (`self.HonkSound`) false))
    (`self.DestroyCheck`)))

(event `self.ReceiveBeginPlay`)

(fn `DestroyCheck`
  (bind (_returnvalue_x _returnvalue_y) (`KismetMathLibrary.BreakVector` (`self.K2_GetActorLocation`)))
  (bind (_returnvalue_x_2 _returnvalue_y_2) (`KismetMathLibrary.BreakVector` (`self.K2_GetActorLocation`)))
  (if (`self.Direction`)
    (if (>= _returnvalue_y (`self.Destination`))
      (`self.K2_DestroyActor`))
    (elif (<= _returnvalue_y_2 (`self.Destination`))
      (`self.K2_DestroyActor`))))

(fn `SetupCar`
  (bind _staticmesh (`self.StaticMesh`))
  (switch `int` (`KismetMathLibrary.RandomIntegerInRange` 0 1)
    (:`0`
      (switch `int` (`KismetMathLibrary.RandomIntegerInRange` 0 1)
        (:`0`
          (`StaticMeshComponent.SetStaticMesh` _staticmesh "/Game/CrossyRoad/Meshes/Vehicles/Short_Car/car.car"))
        (:`1`
          (`StaticMeshComponent.SetStaticMesh` _staticmesh "/Game/CrossyRoad/Meshes/Vehicles/Short_Car_Green/car_green.car_green"))))
    (:`1`
      (switch `int` (`KismetMathLibrary.RandomIntegerInRange` 0 3)
        (:`0`
          (`StaticMeshComponent.SetStaticMesh` _staticmesh "/Game/CrossyRoad/Meshes/Vehicles/Long_Car/long_car.long_car"))
        (:`1`
          (`StaticMeshComponent.SetStaticMesh` _staticmesh "/Game/CrossyRoad/Meshes/Vehicles/Long_Car_Green/long_car_green.long_car_green"))
        (:`2`
          (`StaticMeshComponent.SetStaticMesh` _staticmesh "/Game/CrossyRoad/Meshes/Vehicles/Long_Car_Purple/long_car_purple.long_car_purple"))
        (:`3`
          (`StaticMeshComponent.SetStaticMesh` _staticmesh "/Game/CrossyRoad/Meshes/Vehicles/Long_Car_Police/long_car_police.long_car_police")))))
  (if (`self.Direction`)
    (set `self.Speed` 3.5)
    (set `self.Destination` 610.0)
    (else
      (set `self.Speed` -3.5)
      (set `self.Destination` -550.0)
      (`SceneComponent.K2_AddLocalRotation` (`self.StaticMesh`) (struct :`Yaw` 180.0) false false))))

(fn `UserConstructionScript`)