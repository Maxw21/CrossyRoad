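; Truck obstacle for a Crossy Road-style game that drives along the Y axis and destroys itself at the end of its run.
; SetupTruck, not called within this Blueprint, picks one of three truck meshes at random and uses Direction to set speed, destination and mesh facing.
; Tick applies a fixed local offset each frame, unscaled by delta time, then DestroyCheck compares world Y against the destination.
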(event `self.ReceiveTick`
  (params (DeltaSeconds :type "Float (single-precision)"))
  (`self.K2_AddActorLocalOffset` (`KismetMathLibrary.MakeVector` 0.0 (`self.Speed`)))
  (`self.DestroyCheck`))

(fn `DestroyCheck`
  (bind (_returnvalue_x _returnvalue_y) (`KismetMathLibrary.BreakVector` (`self.K2_GetActorLocation`)))
  (bind (_returnvalue_x_2 _returnvalue_y_2) (`KismetMathLibrary.BreakVector` (`self.K2_GetActorLocation`)))
  (if (`self.Direction`)
    (if (>= _returnvalue_y (`self.Destination`))
      (`self.K2_DestroyActor`))
    (elif (<= _returnvalue_y_2 (`self.Destination`))
      (`self.K2_DestroyActor`))))

(fn `SetupTruck`
  (bind _staticmesh (`self.StaticMesh`))
  (switch `int` (`KismetMathLibrary.RandomIntegerInRange` 0 2)
    (:`0`
      (`StaticMeshComponent.SetStaticMesh` _staticmesh "/Game/CrossyRoad/Meshes/Vehicles/Truck/truck.truck"))
    (:`1`
      (`StaticMeshComponent.SetStaticMesh` _staticmesh "/Game/CrossyRoad/Meshes/Vehicles/Truck_Blue/truck_blue.truck_blue"))
    (:`2`
      (`StaticMeshComponent.SetStaticMesh` _staticmesh "/Game/CrossyRoad/Meshes/Vehicles/Truck_Purple/truck_purple.truck_purple")))
  (if (`self.Direction`)
    (set `self.Speed` 3.5)
    (set `self.Destination` 1000.0)
    (else
      (set `self.Speed` -3.5)
      (set `self.Destination` -1000.0)
      (`SceneComponent.K2_AddLocalRotation` (`self.StaticMesh`) (struct :`Yaw` 180.0) false false))))

(fn `UserConstructionScript`)