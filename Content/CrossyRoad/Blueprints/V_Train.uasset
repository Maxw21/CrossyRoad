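; V_Train is the train in a Crossy Road-style game, crossing along the Y axis until it leaves the play area.
; SetupTrain uses Direction to set a signed speed and end point; Tick applies that speed as a frame-rate-dependent local offset.
; Tick also activates the train sound when the player pawn is close in X and Y.
; DestroyCheck destroys the train past its destination and resets its linked TrainPost.
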(event `self.ReceiveTick`
  (params (DeltaSeconds :type "Float (single-precision)"))
  (bind (_returnvalue_x _returnvalue_y) (`KismetMathLibrary.BreakVector` (`self.K2_GetActorLocation`)))
  (bind (_returnvalue_x_2 _returnvalue_y_2) (`KismetMathLibrary.BreakVector` (`self.K2_GetActorLocation` (`GameplayStatics.GetPlayerPawn` 0))))
  (`self.K2_AddActorLocalOffset` (`KismetMathLibrary.MakeVector` 0.0 (`self.Speed`)))
  (if (and (`KismetMathLibrary.NearlyEqual_FloatFloat` _returnvalue_x _returnvalue_x_2 45.0) (`KismetMathLibrary.NearlyEqual_FloatFloat` _returnvalue_y _returnvalue_y_2 45.0))
    (`ActorComponent.Activate` (`self.TrainSound`) false))
  (`self.DestroyCheck`))

(fn `DestroyCheck`
  (bind (_returnvalue_x _returnvalue_y) (`KismetMathLibrary.BreakVector` (`self.K2_GetActorLocation`)))
  (bind (_returnvalue_x_2 _returnvalue_y_2) (`KismetMathLibrary.BreakVector` (`self.K2_GetActorLocation`)))
  (bind _trainpost (`self.TrainPost`))
  (if (`self.Direction`)
    (if (>= _returnvalue_y (`self.Destination`))
      (`self.K2_DestroyActor`)
      (`/Engine/EditorBlueprintResources/StandardMacros.IsValid` _trainpost
        (:`Is Valid`
          (`/Game/CrossyRoad/Blueprints/Train_Post.ResetPost` _trainpost))))
    (elif (<= _returnvalue_y_2 (`self.Destination`))
      (`self.K2_DestroyActor`)
      (`/Engine/EditorBlueprintResources/StandardMacros.IsValid` _trainpost
        (:`Is Valid`
          (`/Game/CrossyRoad/Blueprints/Train_Post.ResetPost` _trainpost))))))

(fn `SetupTrain`
  (if (`self.Direction`)
    (set `self.Speed` 30.0)
    (set `self.Destination` 1200.0)
    (else
      (set `self.Speed` -30.0)
      (set `self.Destination` -1200.0))))

(fn `UserConstructionScript`)