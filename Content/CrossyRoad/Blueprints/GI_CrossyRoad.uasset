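; Game instance Blueprint for Crossy Road that saves and loads the player's coins and high score through SaveCR save objects.
; SaveGame writes both values to a new SaveCR and stores it in that object's default slot and user index.
; LoadGame creates a temporary SaveCR to get the slot, then copies the loaded values onto the player's Chicken pawn, stopping if either cast fails.
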(fn `LoadGame`
  (bind _returnvalue (`GameplayStatics.CreateSaveGameObject` "/Game/CrossyRoad/Blueprints/SaveCR.SaveCR_C"))
  (bind _output_get (set `self.SaveGameInstance` _returnvalue))
  (bind _returnvalue_2 (`GameplayStatics.LoadGameFromSlot` (`/Game/CrossyRoad/Blueprints/SaveCR.SaveSlotName` _output_get) (`/Game/CrossyRoad/Blueprints/SaveCR.UserIndex` _output_get)))
  (bind _assave_cr (cast `/Game/CrossyRoad/Blueprints/SaveCR` _returnvalue_2))
  (bind _output_get_2 (set `self.SaveGameInstance` _assave_cr))
  (bind _aschicken (cast `/Game/CrossyRoad/Blueprints/Chicken` (`GameplayStatics.GetPlayerPawn` 0)))
  (set `/Game/CrossyRoad/Blueprints/Chicken.CoinsCollected` (`/Game/CrossyRoad/Blueprints/SaveCR.Coins` _output_get_2) _aschicken)
  (set `/Game/CrossyRoad/Blueprints/Chicken.HighScore` (`/Game/CrossyRoad/Blueprints/SaveCR.HighScore` _output_get_2) _aschicken))

(fn `SaveGame`
  (params (Coins :type Integer) (HighScore :type Integer))
  (bind _returnvalue (`GameplayStatics.CreateSaveGameObject` "/Game/CrossyRoad/Blueprints/SaveCR.SaveCR_C"))
  (bind _output_get (set `self.SaveGameInstance` _returnvalue))
  (set `/Game/CrossyRoad/Blueprints/SaveCR.Coins` Coins _output_get)
  (set `/Game/CrossyRoad/Blueprints/SaveCR.HighScore` HighScore _output_get)
  (`GameplayStatics.SaveGameToSlot` _output_get (`/Game/CrossyRoad/Blueprints/SaveCR.SaveSlotName` _output_get) (`/Game/CrossyRoad/Blueprints/SaveCR.UserIndex` _output_get)))