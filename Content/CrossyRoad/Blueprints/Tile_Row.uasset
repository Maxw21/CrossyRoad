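; Tile_Row is one terrain strip in a Crossy Road-style game: grass, road, water or railroad.
; SetupRow sets its meshes and spawns random scenery and coins, lily pads, a train post or a vehicle spawner by type, with GrassColor varying grass and water rows.
; Overlap pushes the Chicken back at the side limits.
; DestroyRow removes the row and its spawner once the player is far enough ahead.
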(event `self.ReceiveBeginPlay`)

(event `self.ReceiveActorBeginOverlap`
  (params (OtherActor :type "Actor Object Reference"))
  (bind _aschicken (cast `/Game/CrossyRoad/Blueprints/Chicken` OtherActor))
  (bind (_returnvalue_x _returnvalue_y) (`KismetMathLibrary.BreakVector` (`self.K2_GetActorLocation` _aschicken)))
  (if (>= _returnvalue_y 480.0)
    (bind _rootcomponent (`Actor.RootComponent` _aschicken))
    (bind (_returnvalue_x_2 _returnvalue_y_2 _returnvalue_z) (`KismetMathLibrary.BreakVector` (`SceneComponent.K2_GetComponentLocation` _rootcomponent)))
    (`SceneComponent.K2_SetWorldLocation` _rootcomponent (`KismetMathLibrary.MakeVector` _returnvalue_x_2 510.0 _returnvalue_z) false false)
    (else
      (bind (_returnvalue_x_3 _returnvalue_y_3) (`KismetMathLibrary.BreakVector` (`self.K2_GetActorLocation` _aschicken)))
      (if (<= _returnvalue_y_3 -480.0)
        (bind _rootcomponent_2 (`Actor.RootComponent` _aschicken))
        (bind (_returnvalue_x_4 _returnvalue_y_4 _returnvalue_z_2) (`KismetMathLibrary.BreakVector` (`SceneComponent.K2_GetComponentLocation` _rootcomponent_2)))
        (`SceneComponent.K2_SetWorldLocation` _rootcomponent_2 (`KismetMathLibrary.MakeVector` _returnvalue_x_4 -450.0 _returnvalue_z_2) false false)))))

(fn `DestroyRow`
  (bind _returnvalue_x (`KismetMathLibrary.BreakVector` (`self.K2_GetActorLocation`)))
  (bind _vehiclespawner (`self.VehicleSpawner`))
  (bind _trainpost (`self.TrainPost`))
  (bind _returnvalue_x_2 (`KismetMathLibrary.BreakVector` (`self.K2_GetActorLocation` (`GameplayStatics.GetPlayerPawn` 0))))
  (if (>= _returnvalue_x_2 (+ _returnvalue_x 400.0))
    (`self.K2_DestroyActor`)
    (`/Engine/EditorBlueprintResources/StandardMacros.IsValid` _vehiclespawner
      (:`Is Valid`
        (`self.K2_DestroyActor` _vehiclespawner)
        (`/Engine/EditorBlueprintResources/StandardMacros.IsValid` _trainpost
          (:`Is Valid`
            (`self.K2_DestroyActor` _trainpost)))))))

(fn `SetupRow`
  (params (RowType :type Integer) (RowLocation :type "Float (double-precision)") (GrassColor :type Boolean))
  (bind _rowtype (`self.RowType`))
  (bind _output_get (set `self.RowType` RowType))
  (set `self.RowLocation` RowLocation)
  (switch `int` _output_get
    (:`0`
      (`self.SpawnEnvironment`))
    (:`1`
      (bind _returnvalue (`|SpawnActorFromClass` "/Game/CrossyRoad/Blueprints/Spawner_Vehicle.Spawner_Vehicle_C" (`KismetMathLibrary.MakeTransform` (-300.0 30.0 30.0)) "Undefined" "OverrideRootScale" null null :!label _label))
      (set `/Game/CrossyRoad/Blueprints/Spawner_Vehicle.RowType` (`self.RowType`) _returnvalue)
      (set `/Game/CrossyRoad/Blueprints/Spawner_Vehicle.TileRow` self _returnvalue)
      (set `self.VehicleSpawner` _returnvalue))
    (:`2`
      (if GrassColor
        (if (== (`KismetMathLibrary.RandomIntegerInRange` 0 1) 0)
          (`self.SpawnLilyPads`)
          (else
            (goto _label)))
        (else
          (goto _label))))
    (:`3`
      (`self.SpawnTrainPost`)
      (goto _label)))
  (for _array_element (`self.K2_GetComponentsByClass` "/Script/Engine.StaticMeshComponent")
    (`StaticMeshComponent.SetStaticMesh` _array_element (select `int` _rowtype :`0` "/Game/CrossyRoad/Meshes/Tiles/Grass/grass.grass" :`1` "/Game/CrossyRoad/Meshes/Tiles/Road/road_base.road_base" :`2` "/Game/CrossyRoad/Meshes/Tiles/Water/water.water" :`3` "/Game/CrossyRoad/Meshes/Tiles/Railroad/railroad.railroad" :!type "StaticMesh Object Reference"))
    (if (== _rowtype 0)
      (if GrassColor
        (`StaticMeshComponent.SetStaticMesh` _array_element "/Game/CrossyRoad/Meshes/Tiles/Grass_1/grass1.grass1"))
      (elif (== _rowtype 2)
        (set `PrimitiveComponent.bGenerateOverlapEvents` true _array_element)))))

(fn `SpawnEnvironment`
  (bind _returnvalue (`KismetMathLibrary.Conv_IntToDouble` (+ (* (`KismetMathLibrary.RandomIntegerInRange` -15 15) 40) 30)))
  (for _ (range 3)
    (switch `int` (`KismetMathLibrary.RandomIntegerInRange` 0 2)
      (:`0`
        (bind _returnvalue_2 (`|SpawnActorFromClass` "/Game/CrossyRoad/Blueprints/E_Tree.E_Tree_C" (`KismetMathLibrary.MakeTransform` (`KismetMathLibrary.MakeVector` (`self.RowLocation`) _returnvalue)) "Undefined" "OverrideRootScale" null null))
        (`/Game/CrossyRoad/Blueprints/E_Tree.SetMesh` _returnvalue_2))
      (:`1`
        (`|SpawnActorFromClass` "/Game/CrossyRoad/Blueprints/E_Rock.E_Rock_C" (`KismetMathLibrary.MakeTransform` (`KismetMathLibrary.MakeVector` (`self.RowLocation`) _returnvalue)) "Undefined" "OverrideRootScale" null null))
      (:`2`
        (`|SpawnActorFromClass` "/Game/CrossyRoad/Blueprints/Coin.Coin_C" (`KismetMathLibrary.MakeTransform` (`KismetMathLibrary.MakeVector` (`self.RowLocation`) _returnvalue 5.0)) "Undefined" "OverrideRootScale" null null)))))

(fn `SpawnLilyPads`
  (for _ (range 2)
    (`|SpawnActorFromClass` "/Game/CrossyRoad/Blueprints/E_LilyPad.E_LilyPad_C" (`KismetMathLibrary.MakeTransform` (`KismetMathLibrary.MakeVector` (`self.RowLocation`) (`KismetMathLibrary.Conv_IntToDouble` (+ (* (`KismetMathLibrary.RandomIntegerInRange` -10 10) 40) 30)) 1.5)) "Undefined" "OverrideRootScale" null null)))

(fn `SpawnTrainPost`
  (bind _returnvalue (`|SpawnActorFromClass` "/Game/CrossyRoad/Blueprints/Train_Post.Train_Post_C" (`KismetMathLibrary.MakeTransform` (`KismetMathLibrary.MakeVector` (- (`self.RowLocation`) 20.0) 0.0 3.0)) "Undefined" "OverrideRootScale" null null))
  (set `self.TrainPost` _returnvalue))

(fn `UserConstructionScript`)