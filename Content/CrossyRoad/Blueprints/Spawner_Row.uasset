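; Spawner actor that builds the lane-by-lane level for a Crossy Road-style game from Tile_Row actors.
; On BeginPlay it registers with the Chicken, clears existing rows, then lays a fixed-type starting strip followed by randomized rows.
; Random rows form same-type runs, never repeating the previous type, with length ranges chosen using the Chicken's furthest tile.
; SpawnRowAtSpawnPoint adds one row per call, alternating the grass shade.
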(event `self.ReceiveBeginPlay`
  (bind _aschicken (cast `/Game/CrossyRoad/Blueprints/Chicken` (`GameplayStatics.GetPlayerPawn` 0)))
  (set `/Game/CrossyRoad/Blueprints/Chicken.RowSpawner` self _aschicken)
  (`self.SpawnInitialRows`))

(fn `SpawnInitialRows`
  (`|ExecutionSequence`
    (:`then_0`
      (bind _outactors (`GameplayStatics.GetAllActorsOfClass` "/Game/CrossyRoad/Blueprints/Tile_Row.Tile_Row_C"))
      (for _array_element _outactors
        (`self.K2_DestroyActor` _array_element)))
    (:`then_1`
      (`self.SpawnStartingRows`))
    (:`then_2`
      (for _ (range 26)
        (`self.SpawnRowsWithAmount`)))))

(fn `SpawnRow`
  (params (SpawnLocation :type "Vector Structure") (RowType :type Integer))
  (bind _grasscolor (`self.GrassColor`))
  (bind _returnvalue (`|SpawnActorFromClass` "/Game/CrossyRoad/Blueprints/Tile_Row.Tile_Row_C" (`KismetMathLibrary.MakeTransform` SpawnLocation) "Undefined" "OverrideRootScale" null null))
  (bind _output_get (set `self.NewestRow` _returnvalue))
  (set `/Game/CrossyRoad/Blueprints/Tile_Row.RowSpawner` self _output_get)
  (`/Game/CrossyRoad/Blueprints/Tile_Row.SetupRow` _output_get RowType (`self.NextRowLocation`) _grasscolor)
  (if _grasscolor
    (set `self.GrassColor` false)
    (else
      (set `self.GrassColor` true))))

(fn `SpawnRowAtSpawnPoint`
  (`self.SpawnRowsWithAmount`))

(fn `SpawnRowsWithAmount`
  (bind _currentrowtype (`self.CurrentRowType`))
  (if (`self.GenNewRowType`)
    (bind _aschicken (cast `/Game/CrossyRoad/Blueprints/Chicken` (`GameplayStatics.GetPlayerPawn` 0)))
    (bind _output_get (set `self.CurrentRowType` (`KismetMathLibrary.RandomIntegerInRange` 0 3) :!label _label))
    (if (== _output_get (`self.LastRowType`))
      (goto _label)
      (else
        (set `self.LastRowType` _currentrowtype)
        (bind _returnvalue (`DecideRow.DecideNumOfRows` _currentrowtype (`/Game/CrossyRoad/Blueprints/Chicken.FurthestTileNumber` _aschicken)))
        (switch `int` _returnvalue
          (:`0`
            (set `self.NumOfRows` (`KismetMathLibrary.RandomIntegerInRange` 1 3)))
          (:`1`
            (set `self.NumOfRows` (`KismetMathLibrary.RandomIntegerInRange` 5 10)))
          (:`2`
            (set `self.NumOfRows` (`KismetMathLibrary.RandomIntegerInRange` 10 15)))
          (:`3`
            (set `self.NumOfRows` (`KismetMathLibrary.RandomIntegerInRange` 15 20))))
        (set `self.GenNewRowType` false))))
  (`self.SpawnRow` (`KismetMathLibrary.MakeVector` (`self.NextRowLocation`) 30.0) (`self.CurrentRowType`))
  (set `self.NextRowLocation` (+ (`self.NextRowLocation`) 40.0))
  (bind _result (`/Engine/EditorBlueprintResources/StandardMacros.IncrementInt` (`self.RowCounter`))
    (:`  `
      (bind _output_get_2 (set `self.RowCounter` _result))
      (if (>= _output_get_2 (`self.NumOfRows`))
        (set `self.GenNewRowType` true)
        (set `self.RowCounter` 0)))))

(fn `SpawnStartingRows`
  (bind _grasscolor (`self.GrassColor`))
  (bind _nextrowlocation (`self.NextRowLocation`))
  (for _ (range 19)
    (bind _returnvalue (`|SpawnActorFromClass` "/Game/CrossyRoad/Blueprints/Tile_Row.Tile_Row_C" (`KismetMathLibrary.MakeTransform` (`KismetMathLibrary.MakeVector` (`self.NextRowLocation`) 30.0)) "Undefined" "OverrideRootScale" null null))
    (bind _output_get (set `self.NewestRow` _returnvalue))
    (set `/Game/CrossyRoad/Blueprints/Tile_Row.RowSpawner` self _output_get)
    (`/Game/CrossyRoad/Blueprints/Tile_Row.SetupRow` _output_get 0 _nextrowlocation _grasscolor)
    (set `self.NextRowLocation` (+ _nextrowlocation 40.0))
    (if _grasscolor
      (set `self.GrassColor` false)
      (else
        (set `self.GrassColor` true)))))

(fn `UserConstructionScript`)