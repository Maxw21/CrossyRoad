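; Train crossing signal post for a Crossy Road style game, with two alternating warning lights and a crossing sound.
; While BlinkLights is on, Tick swaps the left and right point lights on a short timer.
; It also activates the sound if SoundOn is set and the player pawn is near the post along the X axis.
; ResetPost clears both flags, stops the sound and hides both lights; nothing here sets those flags true.
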(event `self.ReceiveBeginPlay`
  (`SceneComponent.SetVisibility` (`self.PointLightR`) false false)
  (`SceneComponent.SetVisibility` (`self.PointLightL`) false false))

(event `self.ReceiveTick`
  (params (DeltaSeconds :type "Float (single-precision)"))
  (if (`self.BlinkLights`)
    (`self.PlaySound`)
    (bind _output_get (set `self.BlinkCounter` (+ DeltaSeconds (`self.BlinkCounter`))))
    (if (>= _output_get 0.4)
      (if (`self.FlipLights`)
        (`SceneComponent.SetVisibility` (`self.PointLightR`) false false)
        (`SceneComponent.SetVisibility` (`self.PointLightL`) true false)
        (set `self.FlipLights` false)
        (else
          (`SceneComponent.SetVisibility` (`self.PointLightL`) false false)
          (`SceneComponent.SetVisibility` (`self.PointLightR`) true false)
          (set `self.FlipLights` true)))
      (set `self.BlinkCounter` 0.0))))

(fn `PlaySound`
  (bind _returnvalue_x (`KismetMathLibrary.BreakVector` (`self.K2_GetActorLocation`)))
  (bind _returnvalue_x_2 (`KismetMathLibrary.BreakVector` (`self.K2_GetActorLocation` (`GameplayStatics.GetPlayerPawn` 0))))
  (if (`self.SoundOn`)
    (if (`KismetMathLibrary.NearlyEqual_FloatFloat` _returnvalue_x _returnvalue_x_2 85.0)
      (`ActorComponent.Activate` (`self.CrossingSound`) false))))

(fn `ResetPost`
  (set `self.SoundOn` false)
  (`ActorComponent.Deactivate` (`self.CrossingSound`))
  (set `self.BlinkLights` false)
  (`SceneComponent.SetVisibility` (`self.PointLightL`) false false)
  (`SceneComponent.SetVisibility` (`self.PointLightR`) false false))

(fn `UserConstructionScript`)